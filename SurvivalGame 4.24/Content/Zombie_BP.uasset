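; Zombie enemy that chases the player and deals melee damage with its claws.
; On BeginPlay it issues an AI Move To targeting the first player's pawn.
; Head and Torso component hits apply fixed damage, with the head taking more than the torso.
; Left and right claw overlaps cast to BasicCharacter and apply AttackPower damage to that character.
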(event OnComponentHit(Head)
  (params (HitComponent :type Primitive%20Component%20Object%20Reference) (OtherActor :type Actor%20Object%20Reference) (OtherComp :type Primitive%20Component%20Object%20Reference) (NormalImpulse :type Vector :default "0, 0, 0") (Hit :type Hit%20Result%20Structure%20%28by%20ref%29))
  (Class|BasicCharacter|ApplyDamage 1e+02))

(event OnComponentHit(Torso)
  (params (HitComponent :type Primitive%20Component%20Object%20Reference) (OtherActor :type Actor%20Object%20Reference) (OtherComp :type Primitive%20Component%20Object%20Reference) (NormalImpulse :type Vector :default "0, 0, 0") (Hit :type Hit%20Result%20Structure%20%28by%20ref%29))
  ;[1 1 1] Add an Apply Damage node here following the example above. Reduce the damage for this one
  (Class|BasicCharacter|ApplyDamage 5e+01))

(event OnComponentBeginOverlap(Claw_Left)
  (params (OverlappedComponent :type Primitive%20Component%20Object%20Reference) (OtherActor :type Actor%20Object%20Reference) (OtherComp :type Primitive%20Component%20Object%20Reference) (OtherBodyIndex :type Integer) (bFromSweep :type Boolean) (SweepResult :type Hit%20Result%20Structure%20%28by%20ref%29))
  (bind _asbasic_character (Utilities|Casting|CastToBasicCharacter OtherActor))
  (Class|BasicCharacter|ApplyDamage _asbasic_character (Variables|Default|GetattackPower)))

(event OnComponentBeginOverlap(Claw_Right)
  (params (OverlappedComponent :type Primitive%20Component%20Object%20Reference) (OtherActor :type Actor%20Object%20Reference) (OtherComp :type Primitive%20Component%20Object%20Reference) (OtherBodyIndex :type Integer) (bFromSweep :type Boolean) (SweepResult :type Hit%20Result%20Structure%20%28by%20ref%29))
  (bind _asbasic_character (Utilities|Casting|CastToBasicCharacter OtherActor))
  (Class|BasicCharacter|ApplyDamage _asbasic_character (Variables|Default|GetattackPower)))

(event EventBeginPlay
  (AI|AIMoveTo self "0, 0, 0" (Game|Player|GetPlayerPawn 0) 5.0 false))

(event Collision|EventActorBeginOverlap
  (params (OtherActor :type Actor%20Object%20Reference)))

(event EventTick
  (params (DeltaSeconds :type Float%20%28single-precision%29)))

(fn ConstructionScript)